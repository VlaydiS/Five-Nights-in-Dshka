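; DoorSingle is an interactable single door that swings open or closed each time Interact is called.
; Interact toggles the opening state, then plays or reverses one Timeline whose Alpha lerps the Door component's relative yaw.
; A moving flag ignores further interactions until the Timeline finishes, so a swing cannot be interrupted.
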(event `/Game/FnifFiles/Blueprints/Interfaces/IE_Interactable.Interact`
  (if (not (`self.IsDoorMoving`))
    (set `self.IsDoorMoving` true)
    (bind _output_get (set `self.IsDoorOpening` (not (`self.IsDoorOpening`))))
    (if _output_get
      (bind (_direction _alpha) (`Timeline|Timeline` :!label _label)
        (:`Update`
          (`SceneComponent.K2_SetRelativeRotation` (`self.Door`) (`KismetMathLibrary.MakeRotator` 0.0 0.0 (`KismetMathLibrary.Lerp` 0.0 -85.0 _alpha)) false false)
          (set `self.IsFinished` true))
        (:`Finished`
          (set `self.IsDoorMoving` false)))
      (else
        (goto _label :!via `Reverse`)))))

(fn `UserConstructionScript`)