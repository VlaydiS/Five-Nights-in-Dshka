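; Player character Blueprint handling movement, look, sprint, crouch, jump and movement-based camera shake.
; Holding jump runs a timeline that drives gravity scale and calls Jump, with launch velocity scaled from current speed; release restores default gravity.
; Sprint and crouch set walk speed, and a reversible timeline smoothly resizes the capsule for crouching.
; Tick starts an idle, walk or run camera shake based on velocity and CanJump.
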(event `InputAction|Jump`
  (params (Key :type "Key Structure"))
  (bind _charactermovement (`self.CharacterMovement`))
  (bind _charactermovement_2 (`self.CharacterMovement`))
  ;[1 1 1] Jumping
  (:`Pressed`
    (bind (_direction _alpha) (`Timeline|JumpTimeline` :!label _label)
      (:`Update`
        (set `CharacterMovementComponent.GravityScale` _alpha _charactermovement_2)
        (set `CharacterMovementComponent.JumpZVelocity` (`self.Select Jump Velocity` _charactermovement) _charactermovement_2)
        (`self.Jump`))))
  (:`Released`
    (`|ExecutionSequence`
      (:`then_0`
        (goto _label :!via `Stop`))
      (:`then_1`
        (set `CharacterMovementComponent.GravityScale` (`self.Default Gravity`) _charactermovement)
        (`self.StopJumping`)))))

(event `InputAction|Sprint`
  (params (Key :type "Key Structure"))
  (bind _charactermovement (`self.CharacterMovement`))
  (bind _is_crouching (`self.Is Crouching`))
  ;[1 1 1] Sprinting
  (:`Pressed`
    (if _is_crouching
      (set `CharacterMovementComponent.MaxWalkSpeed` 250.0 _charactermovement)
      (else
        (set `CharacterMovementComponent.MaxWalkSpeed` 600.0 _charactermovement))))
  (:`Released`
    (if _is_crouching
      (set `CharacterMovementComponent.MaxWalkSpeed` 120.0 _charactermovement)
      (else
        (set `CharacterMovementComponent.MaxWalkSpeed` 300.0 _charactermovement)))))

(event `InputAction|Crouch`
  (params (Key :type "Key Structure"))
  (bind _charactermovement (`self.CharacterMovement`))
  ;[1 1 1] Crouching
  (:`Pressed`
    (set `CharacterMovementComponent.MaxWalkSpeed` 120.0 _charactermovement)
    (set `self.Is Crouching` true)
    (bind (_direction _alpha) (`Timeline|CrouchTimeline` :!label _label_2)
      (:`Update`
        (`CapsuleComponent.SetCapsuleHalfHeight` (`self.CapsuleComponent`) (`KismetMathLibrary.Lerp` 88.0 44.0 _alpha) true))))
  (:`Released`
    (set `CharacterMovementComponent.MaxWalkSpeed` 300.0 _charactermovement)
    (set `self.Is Crouching` false)
    (goto _label_2 :!via `Reverse`)))

(event `InputAxis|MoveForwardBackward`
  (params (AxisValue :type "Float (single-precision)"))
  ;[1 1 1] Keyboard Control
  (`self.AddMovementInput` (`self.GetActorForwardVector`) AxisValue))

(event `InputAxis|LookHorizontal`
  (params (AxisValue :type "Float (single-precision)"))
  ;[1 1 1] Camera control
  (`self.AddControllerYawInput` AxisValue))

(event `InputAxis|LookVertical`
  (params (AxisValue :type "Float (single-precision)"))
  ;[1 1 1] Camera control
  (`self.AddControllerPitchInput` (* AxisValue -1.0)))

(event `InputAxis|MoveLeftRight`
  (params (AxisValue :type "Float (single-precision)"))
  ;[1 1 1] Keyboard Control
  (`self.AddMovementInput` (`self.GetActorRightVector`) AxisValue))

(event `Camera Shake`
  (bind _returnvalue (`GameplayStatics.GetPlayerController` 0))
  (bind _returnvalue_2 (`KismetMathLibrary.VSize` (`self.GetVelocity`)))
  ;[1 1 1] Camera Shake
  (if (and (> _returnvalue_2 0.0) (`self.CanJump`))
    (if (< _returnvalue_2 600.0)
      (`PlayerController.ClientStartCameraShake` :`self` _returnvalue :`Shake` "/Game/Blueprints/Camera/CameraShake_Walk.CameraShake_Walk_C")
      (else
        (`PlayerController.ClientStartCameraShake` :`self` _returnvalue :`Shake` "/Game/Blueprints/Camera/CameraShake_Run.CameraShake_Run_C")))
    (else
      (`PlayerController.ClientStartCameraShake` :`self` _returnvalue :`Shake` "/Game/Blueprints/Camera/CameraShake_Idle.CameraShake_Idle_C"))))

(event `self.ReceiveTick`
  (params (DeltaSeconds :type "Float (single-precision)"))
  ;[1 1 1] Camera Shake
  (`self.Camera Shake`))

(fn `Select Jump Velocity`
  (params (self2 :type "MovementComponent Object Reference"))
  (returns (ReturnValue :type "Float (single-precision)"))
  (bind _returnvalue (`KismetMathLibrary.VSize` (`MovementComponent.Velocity` self2)))
  (return (select `bool` (< _returnvalue 50.0) :`false` (* _returnvalue 0.8) :`true` 350.0 :!type "Float (single-precision)")))

(fn `UserConstructionScript`)