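; Player character Blueprint handling movement, look, sprint, crouch, jump, camera shake and interaction.
; Timelines drive a held jump (gravity scale, speed-based launch velocity) and crouch capsule resizing; sprint and crouch set walk speed.
; Tick plays idle, walk or run shakes by velocity and traces from the camera, toggling FloatHUD over IE_Interactable actors.
; Interact sends InteractMessage to the traced actor, and BeginPlay creates both HUD widgets.
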(event `InputAction|Jump`
  (params (Key :type "Key Structure"))
  (bind _charactermovement (`self.CharacterMovement`))
  (bind _charactermovement_2 (`self.CharacterMovement`))
  ;[1 1 1] Jumping
  (:`Pressed`
    (bind (_direction _alpha) (`Timeline|JumpTimeline` :!label _label)
      (:`Update`
        (set `CharacterMovementComponent.GravityScale` _alpha _charactermovement_2)
        (set `CharacterMovementComponent.JumpZVelocity` (`self.Select Jump Velocity` _charactermovement) _charactermovement_2)
        (`self.Jump`))))
  (:`Released`
    (`|ExecutionSequence`
      (:`then_0`
        (goto _label :!via `Stop`))
      (:`then_1`
        (set `CharacterMovementComponent.GravityScale` (`self.DefaultGravity`) _charactermovement)
        (`self.StopJumping`)))))

(event `InputAction|Crouch`
  (params (Key :type "Key Structure"))
  (bind _charactermovement (`self.CharacterMovement`))
  ;[1 1 1] Crouching
  (:`Pressed`
    (set `CharacterMovementComponent.MaxWalkSpeed` 120.0 _charactermovement)
    (set `self.IsCrouching` true)
    (bind (_direction _alpha) (`Timeline|CrouchTimeline` :!label _label_2)
      (:`Update`
        (`CapsuleComponent.SetCapsuleHalfHeight` (`self.CapsuleComponent`) (`KismetMathLibrary.Lerp` 88.0 30.0 _alpha) true))))
  (:`Released`
    (set `CharacterMovementComponent.MaxWalkSpeed` 300.0 _charactermovement)
    (set `self.IsCrouching` false)
    (goto _label_2 :!via `Reverse`)))

(event `InputAxis|LookHorizontal`
  (params (AxisValue :type "Float (single-precision)"))
  ;[1 1 1] Camera control
  (`self.AddControllerYawInput` AxisValue))

(event `InputAxis|LookVertical`
  (params (AxisValue :type "Float (single-precision)"))
  ;[1 1 1] Camera control
  (`self.AddControllerPitchInput` (* AxisValue -1.0)))

(event `InputAxis|MoveForwardBackward`
  (params (AxisValue :type "Float (single-precision)"))
  ;[1 1 1] Keyboard Control
  (`self.AddMovementInput` (`self.GetActorForwardVector`) AxisValue))

(event `InputAxis|MoveLeftRight`
  (params (AxisValue :type "Float (single-precision)"))
  ;[1 1 1] Keyboard Control
  (`self.AddMovementInput` (`self.GetActorRightVector`) AxisValue))

(event `Camera Shake`
  (bind _returnvalue (`GameplayStatics.GetPlayerController` 0))
  (bind _returnvalue_2 (`KismetMathLibrary.VSize` (`self.GetVelocity`)))
  ;[1 1 1] Camera Shake
  (if (and (> _returnvalue_2 0.0) (`self.CanJump`))
    (if (< _returnvalue_2 600.0)
      (`PlayerController.ClientStartCameraShake` :`self` _returnvalue :`Shake` "/Game/FnidFiles/Blueprints/Camera/CameraShake_Walk.CameraShake_Walk_C")
      (else
        (`PlayerController.ClientStartCameraShake` :`self` _returnvalue :`Shake` "/Game/FnidFiles/Blueprints/Camera/CameraShake_Run.CameraShake_Run_C")))
    (else
      (`PlayerController.ClientStartCameraShake` :`self` _returnvalue :`Shake` "/Game/FnidFiles/Blueprints/Camera/CameraShake_Idle.CameraShake_Idle_C"))))

(event `InputAction|Sprint`
  (params (Key :type "Key Structure"))
  (bind _charactermovement (`self.CharacterMovement`))
  (bind _iscrouching (`self.IsCrouching`))
  ;[1 1 1] Sprinting
  (:`Pressed`
    (if _iscrouching
      (set `CharacterMovementComponent.MaxWalkSpeed` 250.0 _charactermovement)
      (else
        (set `CharacterMovementComponent.MaxWalkSpeed` 600.0 _charactermovement))))
  (:`Released`
    (if _iscrouching
      (set `CharacterMovementComponent.MaxWalkSpeed` 120.0 _charactermovement)
      (else
        (set `CharacterMovementComponent.MaxWalkSpeed` 300.0 _charactermovement)))))

(event `InputAction|Interact`
  (params (Key :type "Key Structure"))
  (:`Pressed`
    (bind _outhit (`self.GetInteractRay`)
      (:`True`
        (message `/Game/FnidFiles/Blueprints/Interfaces/IE_Interactable.Interact` (`.HitActor` (`GameplayStatics.BreakHitResult` _outhit)))))))

(event `self.ReceiveBeginPlay`
  (`|ExecutionSequence`
    (:`then_0`
      ;[1 1 1] UI
      (bind _returnvalue (`|CreateWidget` "/Game/FnidFiles/UI/FloatHUD.FloatHUD_C"))
      (set `self.FloatHUD` _returnvalue))
    (:`then_1`
      (bind _returnvalue_2 (`|CreateWidget` "/Game/FnidFiles/UI/GameHUD.GameHUD_C"))
      (`UserWidget.AddToViewport` _returnvalue_2 0))))

(event `self.ReceiveTick`
  (params (DeltaSeconds :type "Float (single-precision)"))
  (bind _floathud (`self.FloatHUD`))
  (`|ExecutionSequence`
    (:`then_0`
      (`self.Camera Shake`))
    (:`then_1`
      (bind _outhit (`self.GetInteractRay`)
        (:`True`
          (if (`KismetSystemLibrary.DoesImplementInterface` (`.HitActor` (`GameplayStatics.BreakHitResult` _outhit)) "/Game/FnidFiles/Blueprints/Interfaces/IE_Interactable.IE_Interactable_C")
            (if (not (`Widget.IsInViewport` _floathud))
              (`UserWidget.AddToViewport` _floathud 0))
            (else
              (`Widget.RemoveFromParent` _floathud :!label _label_3))))
        (:`False`
          (goto _label_3))))))

(fn `Select Jump Velocity`
  (params (self2 :type "MovementComponent Object Reference"))
  (returns (ReturnValue :type "Float (single-precision)"))
  (bind _returnvalue (`KismetMathLibrary.VSize` (`MovementComponent.Velocity` self2)))
  (return (select `bool` (< _returnvalue 50.0) :`false` (* _returnvalue 0.8) :`true` 350.0 :!type "Float (single-precision)")))

(fn `UserConstructionScript`)